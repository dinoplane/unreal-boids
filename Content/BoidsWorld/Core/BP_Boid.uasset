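; BP_Boid is a boid actor that moves itself each tick using steering forces.
; Tick takes an acceleration from GetForceVector, whose logic is not in these graphs, and adds it unscaled to Velocity.
; The delta-time-scaled step, rather than Velocity itself, is clamped to MaxSpeed and added to the Cone mesh's world location.
; The actor teleport-free, unswept transform update also faces it along Velocity.
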(event `self.ReceiveTick`
  (params (DeltaSeconds :type "Float (single-precision)"))
  ;[1 1 1] Compute accelerations from steering behaviors
  (bind _returnvalue (`self.GetForceVector`))
  (bind _output_get (set `self.acceleration` _returnvalue))
  ;[1 1 1] Compute movement from velocity and time
  (bind _output_get_2 (set `self.velocity` (+ _output_get (`self.velocity`))))
  ;[1 1 1] Add to current position
  (`self.K2_SetActorTransform` (`KismetMathLibrary.MakeTransform` (+ (`KismetMathLibrary.ClampVectorSize` (* (`GameplayStatics.GetWorldDeltaSeconds`) _output_get_2 2.0) 0.0 (`self.maxSpeed`)) (.location (`SceneComponent.K2_GetComponentToWorld` (`self.Cone`)))) (`KismetMathLibrary.MakeRotFromX` (`self.velocity`)))))

(fn `UserConstructionScript`)